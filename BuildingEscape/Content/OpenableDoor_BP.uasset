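; Openable door actor that swings open and closed in response to the OpenDoor OnOpen and OnClose events.
; BeginPlay caches the starting rotation and location.
; A timeline plays forward to open and reverses to close, adding its OpenAngle track as a yaw offset to the initial rotation of the whole actor.
; The timeline's Sound Timing event track plays the Doorlock sound at the cached location.
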(event OnOpen(OpenDoor)
  (bind _openangle (Timeline|Timeline_0 Play)
    (:Update
      (Transformation|SetActorRotation (Math|Rotator|CombineRotators (Math|Rotator|MakeRotator 0.0 0.0 _openangle) (Variables|Default|GetInitialRotation))))
    (:SoundTiming
      (Audio|PlaySoundatLocation "/Game/Audio/door-lock.door-lock" (Variables|Default|GetDoorLocation)))))

(event OnClose(OpenDoor)
  (bind _openangle (Timeline|Timeline_0 Reverse)
    (:Update
      (Transformation|SetActorRotation (Math|Rotator|CombineRotators (Math|Rotator|MakeRotator 0.0 0.0 _openangle) (Variables|Default|GetInitialRotation))))
    (:SoundTiming
      (Audio|PlaySoundatLocation "/Game/Audio/door-lock.door-lock" (Variables|Default|GetDoorLocation)))))

(event EventBeginPlay
  (Variables|Default|SetInitialRotation (Transformation|GetActorRotation))
  (Variables|Default|SetDoorLocation (Transformation|GetActorLocation)))

(fn ConstructionScript)